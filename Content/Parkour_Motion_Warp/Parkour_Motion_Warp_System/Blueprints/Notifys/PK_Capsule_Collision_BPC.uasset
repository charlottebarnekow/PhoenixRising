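; Anim notify state for the parkour motion warp system that changes the owner's capsule collision during an animation window.
; On begin and on end it finds the Parkour_Component_BPC on the mesh owner and sets one channel response on that component's capsule.
; Each edge uses its own channel and response variables, so the end sets a specified value rather than restoring a cached one.
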(fn ReceivedNotifyBegin
  (params (MeshComp :type Skeletal%20Mesh%20Component%20Object%20Reference) (Animation :type Anim%20Sequence%20Base%20Object%20Reference) (TotalDuration :type Float%20%28single-precision%29))
  (bind _returnvalue (Components|GetOwner MeshComp))
  (bind _returnvalue_2 (Actor|GetComponentbyClass _returnvalue "/Game/Parkour_Motion_Warp/Parkour_Motion_Warp_System/Blueprints/Parkour_Component_BPC.Parkour_Component_BPC_C"))
  (Utilities|IsValid _returnvalue_2
    (:Is%20Valid
      (Collision|SetCollisionResponsetoChannel (Variables|/Game/Parkour_Motion_Warp/Parkour_Motion_Warp_System/Blueprints/Parkour_Component_BPC.Parkour_Component_BPC_C|GetCapsule%20Component _returnvalue_2) (Variables|Default|GetChannel_Start) (Variables|Default|GetNew%20Response_Start))
      (return false))))

(fn ReceivedNotifyEnd
  (params (MeshComp :type Skeletal%20Mesh%20Component%20Object%20Reference) (Animation :type Anim%20Sequence%20Base%20Object%20Reference))
  (bind _returnvalue (Components|GetOwner MeshComp))
  (bind _returnvalue_2 (Actor|GetComponentbyClass _returnvalue "/Game/Parkour_Motion_Warp/Parkour_Motion_Warp_System/Blueprints/Parkour_Component_BPC.Parkour_Component_BPC_C"))
  (Utilities|IsValid _returnvalue_2
    (:Is%20Valid
      (Collision|SetCollisionResponsetoChannel (Variables|/Game/Parkour_Motion_Warp/Parkour_Motion_Warp_System/Blueprints/Parkour_Component_BPC.Parkour_Component_BPC_C|GetCapsule%20Component _returnvalue_2) (Variables|Default|GetChannel_End) (Variables|Default|GetNew%20Response_End))
      (return false))))