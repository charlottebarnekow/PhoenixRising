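; Animation notify for the parkour system that switches the owning character's movement mode at a point in an animation, presumably to toggle flying during moves.
; It finds the Parkour_Component_BPC on the mesh's owner and applies the notify's NewMovementMode through that component's character movement reference.
; When the resulting mode is Falling or Walking, it clears the component's vault, climb and object-hit flags.
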(fn ReceivedNotify
  (params (MeshComp :type Skeletal%20Mesh%20Component%20Object%20Reference) (Animation :type Anim%20Sequence%20Base%20Object%20Reference))
  (bind _returnvalue (Components|GetOwner MeshComp))
  (bind _returnvalue_2 (Actor|GetComponentbyClass _returnvalue "/Game/Parkour_Motion_Warp/Parkour_Motion_Warp_System/Blueprints/Parkour_Component_BPC.Parkour_Component_BPC_C"))
  (bind _character_movement_component (Variables|/Game/Parkour_Motion_Warp/Parkour_Motion_Warp_System/Blueprints/Parkour_Component_BPC.Parkour_Component_BPC_C|GetCharacter%20Movement%20Component _returnvalue_2))
  (bind _movementmode (Variables|/Script/Engine.CharacterMovementComponent|GetMovementMode _character_movement_component))
  (Utilities|IsValid _returnvalue_2
    (:Is%20Valid
      (Pawn|Components|CharacterMovement|SetMovementMode _character_movement_component (Variables|Default|GetNew%20Movement%20Mode) 0)
      (if (or (Utilities|Enum|Equal(Enum) _movementmode "MOVE_Falling") (Utilities|Enum|Equal(Enum) _movementmode "MOVE_Walking"))
        (Variables|/Game/Parkour_Motion_Warp/Parkour_Motion_Warp_System/Blueprints/Parkour_Component_BPC.Parkour_Component_BPC_C|SetCanVault? _returnvalue_2 false)
        (Variables|/Game/Parkour_Motion_Warp/Parkour_Motion_Warp_System/Blueprints/Parkour_Component_BPC.Parkour_Component_BPC_C|SetCanClimb? _returnvalue_2 false)
        (Variables|/Game/Parkour_Motion_Warp/Parkour_Motion_Warp_System/Blueprints/Parkour_Component_BPC.Parkour_Component_BPC_C|SetObject%20Hit? _returnvalue_2 false)
        (return false)
        (else
          (return false))))))