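; Anim notify state for the parkour system that drives a Bezier-based move to the ground point past an object.
; On begin, it initializes the owner's Parkour component Bezier variables and derives an interp speed from distance to that point over notify duration.
; Each tick calls the component's BezierAlphaCalculate with the notify's offset, speed and debug settings.
; On end, it clears the component's StopMoving flag.
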(fn ReceivedNotifyTick
  (params (MeshComp :type Skeletal%20Mesh%20Component%20Object%20Reference) (Animation :type Anim%20Sequence%20Base%20Object%20Reference) (FrameDeltaTime :type Float%20%28single-precision%29))
  (bind _returnvalue (Components|GetOwner MeshComp))
  (bind _returnvalue_2 (Actor|GetComponentbyClass _returnvalue "/Game/Parkour_Motion_Warp/Parkour_Motion_Warp_System/Blueprints/Parkour_Component_BPC.Parkour_Component_BPC_C"))
  (Utilities|IsValid _returnvalue_2
    (:Is%20Valid
      (Default|BezierAlphaCalculate _returnvalue_2 (Variables|Default|GetFront/%20Back%20Offset) (Variables|Default|GetZ_Offset%20Between%20Points) (Variables|Default|GetInterp%20Speed) (Variables|Default|GetDraw%20Debug%20Sphere%20After%20Object))
      (return false))))

(fn ReceivedNotifyBegin
  (params (MeshComp :type Skeletal%20Mesh%20Component%20Object%20Reference) (Animation :type Anim%20Sequence%20Base%20Object%20Reference) (TotalDuration :type Float%20%28single-precision%29))
  (bind _returnvalue (Components|GetOwner MeshComp))
  (bind _returnvalue_2 (Actor|GetComponentbyClass _returnvalue "/Game/Parkour_Motion_Warp/Parkour_Motion_Warp_System/Blueprints/Parkour_Component_BPC.Parkour_Component_BPC_C"))
  (Utilities|IsValid _returnvalue_2
    (:Is%20Valid
      (Default|SetBezierVariable _returnvalue_2)
      (Variables|/Game/Parkour_Motion_Warp/Parkour_Motion_Warp_System/Blueprints/Parkour_Component_BPC.Parkour_Component_BPC_C|SetNotify_State_Interp%20Speed _returnvalue_2 (/ (/ (Math|Vector|Distance(Vector) (Variables|/Game/Parkour_Motion_Warp/Parkour_Motion_Warp_System/Blueprints/Parkour_Component_BPC.Parkour_Component_BPC_C|GetLastLocationVector _returnvalue_2) (Variables|/Game/Parkour_Motion_Warp/Parkour_Motion_Warp_System/Blueprints/Parkour_Component_BPC.Parkour_Component_BPC_C|GetAfter_Object_Ground_Point _returnvalue_2)) TotalDuration) 1e+02))
      (return false))))

(fn ReceivedNotifyEnd
  (params (MeshComp :type Skeletal%20Mesh%20Component%20Object%20Reference) (Animation :type Anim%20Sequence%20Base%20Object%20Reference))
  (bind _returnvalue (Components|GetOwner MeshComp))
  (bind _returnvalue_2 (Actor|GetComponentbyClass _returnvalue "/Game/Parkour_Motion_Warp/Parkour_Motion_Warp_System/Blueprints/Parkour_Component_BPC.Parkour_Component_BPC_C"))
  (Utilities|IsValid _returnvalue_2
    (:Is%20Valid
      (Variables|/Game/Parkour_Motion_Warp/Parkour_Motion_Warp_System/Blueprints/Parkour_Component_BPC.Parkour_Component_BPC_C|SetStop_Moving _returnvalue_2 false)
      (return false))))